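; LakeWater is a lake water actor that slows the first-person character wading in it and slowly bobs up and down.
; Overlap events on its Cylinder component set the FirstPersonCharacter's max walk speed to a reduced value on entry and a fixed higher value on exit.
; Tick adds a small time-based sine offset to the Cylinder's world Z, an accumulating, frame-rate-dependent motion without delta-time scaling.
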(event `self.Cylinder.OnComponentBeginOverlap`
  (params (OverlappedComponent :type "PrimitiveComponent Object Reference") (OtherActor :type "Actor Object Reference") (OtherComp :type "PrimitiveComponent Object Reference") (OtherBodyIndex :type Integer) (bFromSweep :type Boolean) (SweepResult :type "HitResult Structure (by ref)"))
  (bind _asfirst_person_character (cast `/Game/Blueprints/FirstPersonCharacter` OtherActor))
  (set `CharacterMovementComponent.MaxWalkSpeed` 300.0 (`Character.CharacterMovement` _asfirst_person_character)))

(event `self.Cylinder.OnComponentEndOverlap`
  (params (OverlappedComponent :type "PrimitiveComponent Object Reference") (OtherActor :type "Actor Object Reference") (OtherComp :type "PrimitiveComponent Object Reference") (OtherBodyIndex :type Integer))
  (bind _asfirst_person_character (cast `/Game/Blueprints/FirstPersonCharacter` OtherActor))
  (set `CharacterMovementComponent.MaxWalkSpeed` 600.0 (`Character.CharacterMovement` _asfirst_person_character)))

(event `self.ReceiveTick`
  (params (DeltaSeconds :type "Float (single-precision)"))
  (bind _cylinder (`self.Cylinder`))
  (bind (_returnvalue_x _returnvalue_y _returnvalue_z) (`KismetMathLibrary.BreakVector` (`SceneComponent.K2_GetComponentLocation` _cylinder)))
  (`SceneComponent.K2_SetWorldLocation` _cylinder (`KismetMathLibrary.MakeVector` _returnvalue_x _returnvalue_y (+ _returnvalue_z (/ (`KismetMathLibrary.DegSin` (* (`GameplayStatics.GetTimeSeconds`) 10.0)) 30.0))) false false))

(fn `UserConstructionScript`)